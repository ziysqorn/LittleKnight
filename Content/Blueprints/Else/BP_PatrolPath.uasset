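; BP_PatrolPath is a patrol area actor that keeps its assigned Enemy walking back and forth along the X axis.
; When that Enemy leaves the Box, the actor compares X positions to tell whether it is heading away from the center.
; If so, it halts the Enemy briefly, restores its walk speed and points MovementDirection back inward.
; A DoOnce per side blocks repeat turns during the pause.
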(event `self.Box.OnComponentEndOverlap`
  (params (OverlappedComponent :type "PrimitiveComponent Object Reference") (OtherActor :type "Actor Object Reference") (OtherComp :type "PrimitiveComponent Object Reference") (OtherBodyIndex :type Integer))
  (bind _enemy (`self.Enemy`))
  (bind _enemy_2 (`self.Enemy`))
  (bind _returnvalue_x (`KismetMathLibrary.BreakVector` (- (`self.K2_GetActorLocation`) (`self.K2_GetActorLocation` (`self.Enemy`)))))
  (if (and (`KismetSystemLibrary.IsValid` OtherComp) (`KismetSystemLibrary.IsValid` OtherActor))
    (if (== OtherActor (`self.Enemy`))
      (if (`self.IsActorBeingDestroyed` (`self.Enemy`))
        _
        (elif (> _returnvalue_x 0.0)
          (if (> (`/Game/Blueprints/Characters/Enemy/Knight/BP_Enemy.Movement_Direction` (`self.Enemy`)) 0.0)
            _
            (elif (`KismetSystemLibrary.IsValid` (`self.Enemy`))
              (`/Engine/EditorBlueprintResources/StandardMacros.DoOnce` false :!label _label
                (:`Completed`
                  (set `CharacterMovementComponent.MaxWalkSpeed` 0.0 (`Character.CharacterMovement` (`self.Enemy`)))
                  (`KismetSystemLibrary.Delay` 1.0)
                  (set `CharacterMovementComponent.MaxWalkSpeed` (`/Game/Blueprints/Characters/Enemy/Knight/BP_Enemy.MaxWalkSpeed` _enemy_2) (`Character.CharacterMovement` _enemy_2))
                  (set `/Game/Blueprints/Characters/Enemy/Knight/BP_Enemy.Movement_Direction` 1.0 _enemy_2)
                  (goto _label :!via `Reset`)))))
          (elif (> (`/Game/Blueprints/Characters/Enemy/Knight/BP_Enemy.Movement_Direction` (`self.Enemy`)) 0.0)
            (if (`KismetSystemLibrary.IsValid` (`self.Enemy`))
              (`/Engine/EditorBlueprintResources/StandardMacros.DoOnce` false :!label _label_2
                (:`Completed`
                  (set `CharacterMovementComponent.MaxWalkSpeed` 0.0 (`Character.CharacterMovement` (`self.Enemy`)))
                  (`KismetSystemLibrary.Delay` 1.0)
                  (set `CharacterMovementComponent.MaxWalkSpeed` (`/Game/Blueprints/Characters/Enemy/Knight/BP_Enemy.MaxWalkSpeed` _enemy) (`Character.CharacterMovement` _enemy))
                  (set `/Game/Blueprints/Characters/Enemy/Knight/BP_Enemy.Movement_Direction` -1.0 _enemy)
                  (goto _label_2 :!via `Reset`))))))))))

(fn `UserConstructionScript`)