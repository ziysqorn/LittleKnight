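; BP_CheckPoint is a one-shot checkpoint trigger that saves the player's respawn location and restores health.
; On Box overlap, it stores its own location as BP_Player's LastCheckPoint, sets Health to a fixed value rather than MaxHealth, and updates the health bar through BP_PlayerController.
; DoOnce precedes the player cast, so the first valid overlap by any actor uses up the checkpoint.
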(event `self.Box.OnComponentBeginOverlap`
  (params (OverlappedComponent :type "PrimitiveComponent Object Reference") (OtherActor :type "Actor Object Reference") (OtherComp :type "PrimitiveComponent Object Reference") (OtherBodyIndex :type Integer) (bFromSweep :type Boolean) (SweepResult :type "HitResult Structure (by ref)"))
  (if (and (`KismetSystemLibrary.IsValid` OtherActor) (`KismetSystemLibrary.IsValid` OtherComp))
    (`/Engine/EditorBlueprintResources/StandardMacros.DoOnce` false
      (:`Completed`
        (bind _asbp_player (cast `/Game/Blueprints/Characters/MainCharacter/BP_Player` OtherActor))
        (set `/Game/Blueprints/Characters/MainCharacter/BP_Player.LastCheckPoint` (`self.K2_GetActorLocation`) _asbp_player)
        (bind _output_get (set `/Game/Blueprints/Characters/MainCharacter/BP_Player.Health` 100.0 _asbp_player))
        (bind _asbp_player_controller (cast `/Game/Blueprints/BP_PlayerController` (`Pawn.GetController` _asbp_player)))
        (`/Game/Blueprints/BP_PlayerController.UpdateHealthBar` _asbp_player_controller (/ _output_get (`/Game/Blueprints/Characters/MainCharacter/BP_Player.MaxHealth` _asbp_player)))))))

(fn `UserConstructionScript`)