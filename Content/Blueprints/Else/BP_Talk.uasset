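; BP_Talk is a one-shot dialogue trigger that opens a conversation when BP_Player overlaps its Box.
; On overlap it disables the player's movement, switches to UI-only input and shows the mouse cursor.
; It creates a WB_Dialogue widget if needed, passes it the text lines, talk index and player, then displays the first line.
; A HaveTalked flag blocks repeat triggers.
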(event `self.Box.OnComponentBeginOverlap`
  (params (OverlappedComponent :type "PrimitiveComponent Object Reference") (OtherActor :type "Actor Object Reference") (OtherComp :type "PrimitiveComponent Object Reference") (OtherBodyIndex :type Integer) (bFromSweep :type Boolean) (SweepResult :type "HitResult Structure (by ref)"))
  (bind _dialogue (`self.Dialogue`))
  (if (`self.haveTalked`)
    _
    (elif (and (`KismetSystemLibrary.IsValid` OtherActor) (`KismetSystemLibrary.IsValid` OtherComp))
      (bind _asbp_player (cast `/Game/Blueprints/Characters/MainCharacter/BP_Player` OtherActor))
      (`CharacterMovementComponent.DisableMovement` (`Character.CharacterMovement` _asbp_player))
      (`WidgetBlueprintLibrary.SetInputMode_UIOnlyEx` (`GameplayStatics.GetPlayerController` 0) (`self.Dialogue`))
      (`self.Dialogue`
        (:`then`
          _)
        (:`else`
          (bind _returnvalue (`|CreateWidget` "/Game/UI/WB_Dialogue.WB_Dialogue_C" (`GameplayStatics.GetPlayerController` 0)))
          (set `self.Dialogue` _returnvalue)))
      (set `/Game/UI/WB_Dialogue.Text` (`self.Text`) _dialogue)
      (set `/Game/UI/WB_Dialogue.TalkIndex` (`self.TalkIndex`) _dialogue)
      (set `/Game/UI/WB_Dialogue.Target` _asbp_player _dialogue)
      (`TextBlock.SetText` (`/Game/UI/WB_Dialogue.Talk` _dialogue) (`KismetTextLibrary.Conv_StringToText` (`|GetArrayItem` (`/Game/UI/WB_Dialogue.Text` _dialogue))))
      (`UserWidget.AddToViewport` _dialogue 0)
      (set `PlayerController.bShowMouseCursor` true (`GameplayStatics.GetPlayerController` 0))
      (set `self.haveTalked` true))))

(fn `UserConstructionScript`)