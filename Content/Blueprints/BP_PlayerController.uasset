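; Player controller Blueprint that owns the main on-screen UI widget and relays health updates to it.
; BeginPlay and possession of a BP_Player pawn each create a WB_Main widget, store it as MainCharacterUI and add it to the viewport, without removing any earlier instance.
; UpdateHealthBar passes a health percentage through to the currently stored widget's health bar.
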(event `self.ReceiveBeginPlay`
  (bind _returnvalue (`|CreateWidget` "/Game/UI/WB_Main.WB_Main_C"))
  (bind _output_get (set `self.MainCharacterUI` _returnvalue))
  (`UserWidget.AddToViewport` _output_get 0))

(event `UpdateHealthBar`
  (params (InPercent :type "Float (single-precision)"))
  (`/Game/UI/WB_Main.SetHealthBarInfo` (`self.MainCharacterUI`) InPercent))

(event `self.ReceivePossess`
  (params (PossessedPawn :type "Pawn Object Reference"))
  (cast `/Game/Blueprints/Characters/MainCharacter/BP_Player` PossessedPawn)
  (bind _returnvalue (`|CreateWidget` "/Game/UI/WB_Main.WB_Main_C"))
  (bind _output_get (set `self.MainCharacterUI` _returnvalue))
  (`UserWidget.AddToViewport` _output_get 0))

(fn `UserConstructionScript`)