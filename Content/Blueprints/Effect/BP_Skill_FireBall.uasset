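; BP_Skill_FireBall is a fireball skill actor that damages the first valid target overlapping its Box.
; Only actors implementing BP_Interface whose overlapped component is a capsule count as hits.
; On a hit it sends FireBallHitableMessage, applies one and a half times the player's Damage with player 0's BP_Player as causer, then destroys itself.
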(event `self.Box.OnComponentBeginOverlap`
  (params (OverlappedComponent :type "PrimitiveComponent Object Reference") (OtherActor :type "Actor Object Reference") (OtherComp :type "PrimitiveComponent Object Reference") (OtherBodyIndex :type Integer) (bFromSweep :type Boolean) (SweepResult :type "HitResult Structure (by ref)"))
  ;[0 0 0] Behavior
  (if (`KismetSystemLibrary.DoesImplementInterface` OtherActor "/Game/Blueprints/Interface/BP_Interface.BP_Interface_C")
    (bind _ascapsule_collision (cast `CapsuleComponent` OtherComp))
    (`/Engine/EditorBlueprintResources/StandardMacros.IsValid` _ascapsule_collision
      (:`Is Valid`
        (bind _asbp_player (cast `/Game/Blueprints/Characters/MainCharacter/BP_Player` (`GameplayStatics.GetPlayerCharacter` 0)))
        (message `/Game/Blueprints/Interface/BP_Interface.FireBallHitable` OtherActor)
        (bind _damage (`/Game/Blueprints/Characters/MainCharacter/BP_Player.Damage` _asbp_player))
        (`GameplayStatics.ApplyDamage` OtherActor (+ (* _damage 0.5) _damage) null _asbp_player)
        (`self.K2_DestroyActor`)))))

(fn `FireBallHitable`)

(fn `UserConstructionScript`)