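; Side-scrolling flipbook enemy (Knight folder) that patrols, detects and attacks the player, and heals them when killed by them.
; Tick drives animation and X-axis movement from state flags, reversing at traced obstacles until sensing or overlap spots the player.
; An attack-box timer runs cooldown-gated line-trace strikes.
; Damage updates the health bar, applies knockback, stun and a timeline-driven material flash, then handles death and removal.
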(event `TriggerFlash`
  (params (Multiplier :type "Float (single-precision)" :default 1.0) (Color :type "LinearColor Structure" :default (struct :`R` 1.0 :`G` 1.0 :`B` 1.0 :`A` 1.0)) (PlayRate :type "Float (single-precision)" :default 5.0))
  ;[0 0 0] TriggerFlash
  (`MaterialInstanceDynamic.SetScalarParameterValue` (`self.DynamicSpriteMat`) "FlashMultiplier" Multiplier)
  (`MaterialInstanceDynamic.SetVectorParameterValue` (`self.DynamicSpriteMat`) "FlashColor" Color)
  (`TimelineComponent.SetPlayRate` (`self.FlashMultiplier`) PlayRate)
  (bind (_direction _alpha) (`Timeline|FlashMultiplier` :!via `PlayFromStart`)
    (:`Update`
      (`MaterialInstanceDynamic.SetScalarParameterValue` (`self.DynamicSpriteMat`) "FlashMultiplier" (`KismetMathLibrary.Lerp` 0.0 Multiplier _alpha)))))

(event `self.ReceiveBeginPlay`
  ;[0 0 0] Event Play
  (set `CharacterMovementComponent.MaxWalkSpeed` (`self.MaxWalkSpeed`) (`self.CharacterMovement`))
  (bind _returnvalue (`PrimitiveComponent.CreateDynamicMaterialInstance` (`self.Sprite`) 0 null "None"))
  (set `self.DynamicSpriteMat` _returnvalue)
  (bind _aswb_enemy (cast `/Game/UI/WB_Enemy` (`WidgetComponent.GetUserWidgetObject` (`self.HealthBar`))))
  (set `self.Enemy_HealthBar` _aswb_enemy))

(event `self.ReceiveTick`
  (params (DeltaSeconds :type "Float (single-precision)"))
  (bind (_returnvalue_x _returnvalue_y _returnvalue_z) (`KismetMathLibrary.BreakVector` (`self.K2_GetActorLocation`)))
  (bind _sprite (`self.Sprite`))
  (bind _fb_attack (`self.FB_Attack`))
  ;[0 0 0] Event Tick
  (`self.K2_SetActorLocation` (`KismetMathLibrary.MakeVector` _returnvalue_x 0.0 _returnvalue_z))
  (if (`self.bIsDead`)
    _
    (elif (`self.bIsHurt`)
      (`PaperFlipbookComponent.SetLooping` _sprite false)
      (`PaperFlipbookComponent.SetFlipbook` _sprite (`self.FB_Hurt`))
      (`PaperFlipbookComponent.Play` _sprite)
      (elif (`self.IsAttacking`)
        (`PaperFlipbookComponent.SetFlipbook` (`self.Sprite`) _fb_attack)
        (`KismetSystemLibrary.Delay` (`PaperFlipbook.GetTotalDuration` _fb_attack))
        (set `self.IsAttacking` false)
        (else
          (`self.Animation Update`)
          (`self.Movement Update`))))))

(event `Animation Update`
  (bind _sprite (`self.Sprite`))
  (bind _sprite_2 (`self.Sprite`))
  (bind _sprite_3 (`self.Sprite`))
  ;[0 0 0] Anmation Update
  (if (> (`KismetMathLibrary.VSize` (`MovementComponent.Velocity` (`self.CharacterMovement`))) 0.0)
    (`PaperFlipbookComponent.SetLooping` _sprite true)
    (`PaperFlipbookComponent.SetFlipbook` _sprite (`self.FB_Walk`))
    (if (not (`PaperFlipbookComponent.IsPlaying` _sprite_2))
      (`PaperFlipbookComponent.Play` _sprite_2))
    (else
      (`PaperFlipbookComponent.SetLooping` _sprite true)
      (`PaperFlipbookComponent.SetFlipbook` _sprite (`self.FB_Idle`))
      (if (not (`PaperFlipbookComponent.IsPlaying` _sprite_3))
        (`PaperFlipbookComponent.Play` _sprite_3)))))

(event `Movement Update`
  (bind _returnvalue (`self.K2_GetActorLocation`))
  ;[0 0 0] Movement Update
  (`|ExecutionSequence`
    (:`then_0`
      (if (> (`self.Movement_Direction`) 0.0)
        (`self.K2_SetActorRotation` (struct))
        (else
          (`self.K2_SetActorRotation` (struct :`Yaw` 180.0)))))
    (:`then_1`
      (`self.AddMovementInput` (1.0 0.0 0.0) (`self.Movement_Direction`))
      (bind (_outhit _returnvalue_2) (`KismetSystemLibrary.LineTraceSingle` _returnvalue (+ _returnvalue (* (`self.GetActorForwardVector`) (30.0 0.0 0.0))) "TraceTypeQuery1"))
      (if _returnvalue_2
        (if (not (`self.PlayerSeen`))
          (`/Engine/EditorBlueprintResources/StandardMacros.DoOnce` false :!label _label
            (:`Completed`
              (set `CharacterMovementComponent.MaxWalkSpeed` 0.0 (`self.CharacterMovement`))
              (`KismetSystemLibrary.Delay` 1.0)
              (set `CharacterMovementComponent.MaxWalkSpeed` (`self.MaxWalkSpeed`) (`self.CharacterMovement`))
              (set `self.Movement_Direction` (* (`self.Movement_Direction`) -1.0))
              (goto _label :!via `Reset`))))))))

(event `self.ReceiveAnyDamage`
  (params (Damage :type "Float (single-precision)") (DamageType :type "DamageType Object Reference") (InstigatedBy :type "Controller Object Reference") (DamageCauser :type "Actor Object Reference"))
  (bind _returnvalue (`self.K2_GetActorLocation` DamageCauser))
  (bind _sprite (`self.Sprite`))
  (bind _returnvalue_2 (`PaperFlipbook.GetTotalDuration` (`self.FB_Hurt`)))
  (bind _returnvalue_x (`KismetMathLibrary.BreakVector` (- (`self.K2_GetActorLocation`) (`self.DamageCauserLocation`))))
  (bind _returnvalue_x_2 (`KismetMathLibrary.BreakVector` (- (`self.K2_GetActorLocation`) _returnvalue)))
  (bind _returnvalue_3 (select `bool` (< _returnvalue_x_2 0.0) :`false` 1.0 :`true` -1.0))
  ;[0 0 0] Get Hit
  (set `self.DamageCauserLocation` _returnvalue)
  (bind _output_get (set `self.Health` (- (`self.Health`) Damage)))
  (`/Game/UI/WB_Enemy.SetHealthInfo` (`self.Enemy_HealthBar`) (/ _output_get (`self.MaxHealth`)))
  (if (> Damage 20.0)
    (`self.LaunchCharacter` (`KismetMathLibrary.MakeVector` (* (+ (`self.PushBackDis`) 100.0) _returnvalue_3) 0.0 180.0))
    (else
      (`self.LaunchCharacter` (`KismetMathLibrary.MakeVector` (* (`self.PushBackDis`) _returnvalue_3) 0.0 80.0))))
  (if (<= (`self.Health`) 0.0)
    (set `self.bIsDead` true)
    (bind _asbp_player (cast `/Game/Blueprints/Characters/MainCharacter/BP_Player` DamageCauser))
    (bind _output_get_2 (set `/Game/Blueprints/Characters/MainCharacter/BP_Player.Health` (`KismetMathLibrary.FClamp` (+ (`/Game/Blueprints/Characters/MainCharacter/BP_Player.Health` _asbp_player) 10.0) 0.0 100.0) _asbp_player))
    (bind _asbp_player_controller (cast `/Game/Blueprints/BP_PlayerController` (`self.GetController` _asbp_player)))
    (`/Game/Blueprints/BP_PlayerController.UpdateHealthBar` _asbp_player_controller (/ _output_get_2 (`/Game/Blueprints/Characters/MainCharacter/BP_Player.MaxHealth` _asbp_player)))
    (`self.TriggerFlash` 1.0)
    (`PaperFlipbookComponent.SetLooping` _sprite false)
    (`PaperFlipbookComponent.SetFlipbook` _sprite (`self.FB_Dead`))
    (`ActorComponent.K2_DestroyComponent` (`self.CapsuleComponent`))
    (if (`PaperFlipbookComponent.IsPlaying` _sprite)
      (`KismetSystemLibrary.Delay` 5.0)
      (else
        (`PaperFlipbookComponent.Play` (`self.Sprite`))
        (`KismetSystemLibrary.Delay` 5.0)))
    (`self.K2_DestroyActor`)
    (else
      (set `self.bIsHurt` true)
      (`self.TriggerFlash` 1.0)
      (if (> Damage 20.0)
        (`KismetSystemLibrary.RetriggerableDelay` (+ (+ (`self.Stunt`) _returnvalue_2) 0.8))
        (else
          (`KismetSystemLibrary.RetriggerableDelay` (+ _returnvalue_2 (`self.Stunt`)))))
      (set `self.bIsHurt` false)
      (if (< _returnvalue_x 0.0)
        (set `self.PlayerSeen` true)
        (set `self.Movement_Direction` 1.0)
        (else
          (set `self.PlayerSeen` true)
          (set `self.Movement_Direction` -1.0))))))

(event `/Game/Blueprints/Interface/BP_Interface.FireBallHitable`
  ;[0 0 0] Get Hit
  (`|SpawnActorFromClass` "/Game/Blueprints/Effect/BP_SkillImpact.BP_SkillImpact_C" (`KismetMathLibrary.MakeTransform` (`self.K2_GetActorLocation`) (`SceneComponent.K2_GetComponentRotation` (`self.Sprite`))) "Undefined" "OverrideRootScale" null null))

(event `self.Attack_Box.OnComponentBeginOverlap`
  (params (OverlappedComponent :type "PrimitiveComponent Object Reference") (OtherActor :type "Actor Object Reference") (OtherComp :type "PrimitiveComponent Object Reference") (OtherBodyIndex :type Integer) (bFromSweep :type Boolean) (SweepResult :type "HitResult Structure (by ref)"))
  ;[0 0 0] Attack
  (cast `/Game/Blueprints/Characters/MainCharacter/BP_Player` OtherActor)
  (bind _returnvalue (`KismetSystemLibrary.K2_SetTimerDelegate` (delegate `Attack_Player`) 0.35 true))
  (set `self.Attack_Event` _returnvalue))

(event `Attack_Player`
  (bind _returnvalue (`self.K2_GetActorLocation`))
  ;[0 0 0] Attack
  (if (`self.bIsDead`)
    _
    (elif (not (`self.bIsHurt`))
      (`/Engine/EditorBlueprintResources/StandardMacros.DoOnce` false :!label _label_2
        (:`Completed`
          (set `self.IsAttacking` true)
          (`KismetSystemLibrary.Delay` (`PaperFlipbook.GetTotalDuration` (`self.FB_Attack`)))
          (`|ExecutionSequence`
            (:`then_0`
              (set `self.IsAttacking` false))
            (:`then_1`
              (bind (_outhit _returnvalue_2) (`KismetSystemLibrary.LineTraceSingleForObjects` _returnvalue (+ (* (`self.GetActorForwardVector`) (`KismetMathLibrary.MakeVector` (`self.Attack_Range`))) _returnvalue) (`|MakeArray` "ObjectTypeQuery3" :!type "EObjectTypeQuery Enum")))
              (if _returnvalue_2
                (`|SpawnActorFromClass` "/Game/Blueprints/Effect/BP_HitImpact.BP_HitImpact_C" (`KismetMathLibrary.MakeTransform` (+ (* (`SceneComponent.GetForwardVector` (`self.Sprite`)) (`KismetMathLibrary.MakeVector` (+ (`self.Attack_Range`) 0.0))) (`self.K2_GetActorLocation`)) (`SceneComponent.K2_GetComponentRotation` (`self.Sprite`))) "Undefined" "OverrideRootScale" null null)
                (bind (_bblockinghit _binitialoverlap _time _distance _location _impactpoint _normal _impactnormal _physmat _hitactor) (`GameplayStatics.BreakHitResult` _outhit))
                (if (== _hitactor (`GameplayStatics.GetPlayerCharacter` 0))
                  (`GameplayStatics.ApplyDamage` _hitactor (`self.Damage`) null self)))
              (`KismetSystemLibrary.Delay` (`self.Attack_Cooldown`))
              (goto _label_2 :!via `Reset`))))))))

(event `self.Attack_Box.OnComponentEndOverlap`
  (params (OverlappedComponent :type "PrimitiveComponent Object Reference") (OtherActor :type "Actor Object Reference") (OtherComp :type "PrimitiveComponent Object Reference") (OtherBodyIndex :type Integer))
  ;[0 0 0] Attack
  (cast `/Game/Blueprints/Characters/MainCharacter/BP_Player` OtherActor)
  (`KismetSystemLibrary.K2_ClearAndInvalidateTimerHandle` (`self.Attack_Event`))
  (goto _label_2 :!via `Reset`))

(event `self.PawnSensing.OnSeePawn`
  (params (Pawn :type "Pawn Object Reference"))
  ;[0 0 0] Detection
  (set `self.PlayerSeen` true)
  (`|AIMoveTo` self (0.0 0.0 0.0) (`GameplayStatics.GetPlayerCharacter` 0) 10.0
    (:`then`
      (`KismetSystemLibrary.RetriggerableDelay` 4.0)
      (set `self.PlayerSeen` false))))

(event `self.DetectionBox.OnComponentBeginOverlap`
  (params (OverlappedComponent :type "PrimitiveComponent Object Reference") (OtherActor :type "Actor Object Reference") (OtherComp :type "PrimitiveComponent Object Reference") (OtherBodyIndex :type Integer) (bFromSweep :type Boolean) (SweepResult :type "HitResult Structure (by ref)"))
  ;[0 0 0] Detection
  (if (and (`KismetSystemLibrary.IsValid` OtherActor) (`KismetSystemLibrary.IsValid` OtherComp))
    (bind _asbp_player (cast `/Game/Blueprints/Characters/MainCharacter/BP_Player` OtherActor))
    (set `self.PlayerSeen` true)
    (bind _returnvalue_x (`KismetMathLibrary.BreakVector` (- (`self.K2_GetActorLocation`) (`self.K2_GetActorLocation` _asbp_player))))
    (if (< _returnvalue_x 0.0)
      (set `self.Movement_Direction` 1.0)
      (else
        (set `self.Movement_Direction` -1.0)))))

(event `self.DetectionBox.OnComponentEndOverlap`
  (params (OverlappedComponent :type "PrimitiveComponent Object Reference") (OtherActor :type "Actor Object Reference") (OtherComp :type "PrimitiveComponent Object Reference") (OtherBodyIndex :type Integer))
  ;[0 0 0] Detection
  (if (and (`KismetSystemLibrary.IsValid` null) (`KismetSystemLibrary.IsValid` null))
    (set `self.PlayerSeen` false)))

(fn `UserConstructionScript`)